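; Arkanoid ball actor that moves along its direction each tick and bounces off whatever blocks it.
; Movement uses a swept local offset, reflecting off the hit normal's X and Y only to keep the ball in the scene.
; Guarded setters toggle double-damage and double-speed states, and BeginPlay tints the ball through a dynamic material.
; Overlapping a KillZVolume resets both states, calls CallOnDeath and destroys the ball.
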(event `self.ReceiveActorBeginOverlap`
  (params (OtherActor :type "Actor Object Reference"))
  (cast `KillZVolume` OtherActor)
  (`self.SetDoubleDamage` false)
  (`self.SetDefaultSpeed`)
  (`self.OnDeath`)
  (`self.K2_DestroyActor`))

(event `self.ReceiveBeginPlay`
  (bind _returnvalue (`PrimitiveComponent.CreateDynamicMaterialInstance` (`self.Ball`) 0 null "None"))
  (bind _output_get (set `self.MaterialInstanceBall` _returnvalue))
  (`MaterialInstanceDynamic.SetVectorParameterValue` _output_get (`self.MaterialInstanceParameterBall`) (`self.MaterialInstanceColorBall`)))

(event `self.ReceiveTick`
  (params (DeltaSeconds :type "Float (single-precision)"))
  (bind _sweephitresult (`SceneComponent.K2_AddLocalOffset` (`self.Ball`) (* (* (`self.Direction`) (`self.Speed`)) DeltaSeconds) true false))
  (bind (_bblockinghit _binitialoverlap _time _distance _location _impactpoint _normal) (`GameplayStatics.BreakHitResult` _sweephitresult))
  (if _bblockinghit
    (set `self.Direction` (`KismetMathLibrary.GetReflectionVector` (`self.Direction`) (`KismetMathLibrary.MakeVector` (.x _normal) (.y _normal))))))

(fn `GetInfoDoubleDamage`
  (returns (DoubleDamage :type Boolean))
  (return (`self.IsDoubleDamage`)))

(fn `GetInfoDoubleSpeed`
  (returns (DoubleSpeed :type Boolean))
  (return (`self.IsDoubleSpeed`)))

(fn `SetDefaultSpeed`
  (bind _doublespeed (`self.GetInfoDoubleSpeed`))
  (if _doublespeed
    (set `self.Speed` (/ (`self.Speed`) 2.0))
    (set `self.IsDoubleSpeed` false))
  (return))

(fn `SetDoubleDamage`
  (params (DoubleDamage :type Boolean))
  (if DoubleDamage
    (bind _doubledamage (`self.GetInfoDoubleDamage`))
    (if (not _doubledamage)
      (set `self.IsDoubleDamage` (`local.DoubleDamage`))
      (`KismetSystemLibrary.PrintString` "DoubleDamage ON" true true (struct :`R` 1.0 :`B` 0.127135 :`A` 1.0) 5.0)
      (return))
    (else
      (bind _doubledamage_2 (`self.GetInfoDoubleDamage`))
      (if _doubledamage_2
        (set `self.IsDoubleDamage` (`local.DoubleDamage`))
        (`KismetSystemLibrary.PrintString` "DoubleDamage OFF" true true (struct :`R` 1.0 :`B` 0.009645 :`A` 1.0) 5.0)
        (return)))))

(fn `SetDoubleSpeed`
  (bind _doublespeed (`self.GetInfoDoubleSpeed`))
  (if (not _doublespeed)
    (set `self.Speed` (* (`self.Speed`) 2.0))
    (set `self.IsDoubleSpeed` true))
  (return))

(fn `UserConstructionScript`)