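; Base Arkanoid brick that loses lives when hit by the game ball and may drop a bonus or penalty when broken.
; A dynamic material instance tints the block by remaining lives, from one to four.
; Double-damage balls remove an extra life per hit.
; At zero lives, the Block component is destroyed and a chain of weighted random rolls spawns at most one pickup affecting balls or carriage.
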(event `self.ReceiveBeginPlay`
  (bind _returnvalue (`PrimitiveComponent.CreateDynamicMaterialInstance` (`self.Block`) 0 null "None"))
  (set `self.MaterialInstanceBlock` _returnvalue)
  (`self.SetColour` (`self.Lives`)))

(event `self.ReceiveHit`
  (params (MyComp :type "PrimitiveComponent Object Reference") (Other :type "Actor Object Reference") (OtherComp :type "PrimitiveComponent Object Reference") (bSelfMoved :type Boolean) (HitLocation :type "Vector Structure") (HitNormal :type "Vector Structure") (NormalImpulse :type "Vector Structure") (Hit :type "HitResult Structure (by ref)"))
  (bind _asbp_game_ball (cast `/Game/Arkanoid/Core/Blueprints/BP_GameBall` Other))
  (if (`/Game/Arkanoid/Core/Blueprints/BP_GameBall.IsDoubleDamage` _asbp_game_ball)
    (`/Engine/EditorBlueprintResources/StandardMacros.DecrementInt` (`self.Lives`)
      (:`  `
        _)))
  (bind _result (`/Engine/EditorBlueprintResources/StandardMacros.DecrementInt` (`self.Lives`))
    (:`  `
      (if (<= _result 0)
        (set `self.SpawnTransformLocationBlock` (`SceneComponent.K2_GetComponentLocation` (`self.Block`)))
        (`ActorComponent.K2_DestroyComponent` (`self.Block`))
        (if (`KismetMathLibrary.RandomBoolWithWeight` (`self.DoubleDamageSpawnChance`))
          (`|SpawnActorFromClass` "/Game/Arkanoid/Core/Blueprints/Bonuses/Positive/BP_DoubleDamageBall.BP_DoubleDamageBall_C" (`KismetMathLibrary.MakeTransform` (`self.SpawnTransformLocationBlock`) (struct) (`self.SpawnTransformScaleExtraBall`)) "Undefined" "OverrideRootScale" null null)
          (elif (`KismetMathLibrary.RandomBoolWithWeight` (`self.ExtraBallSpawnChance`))
            (`|SpawnActorFromClass` "/Game/Arkanoid/Core/Blueprints/Bonuses/Positive/BP_ExtraBall.BP_ExtraBall_C" (`KismetMathLibrary.MakeTransform` (`self.SpawnTransformLocationBlock`) (struct) (`self.SpawnTransformScaleExtraBall`)) "Undefined" "OverrideRootScale" null null)
            (elif (`KismetMathLibrary.RandomBoolWithWeight` (`self.DoubleSpeedBallChance`))
              (`|SpawnActorFromClass` "/Game/Arkanoid/Core/Blueprints/Bonuses/Positive/BP_DoubleSpeedBall.BP_DoubleSpeedBall_C" (`KismetMathLibrary.MakeTransform` (`self.SpawnTransformLocationBlock`) (struct) (`self.SpawnTransformScaleExtraBall`)) "Undefined" "OverrideRootScale" null null)
              (elif (`KismetMathLibrary.RandomBoolWithWeight` (`self.DoubleSpeedCarriageChance`))
                (`|SpawnActorFromClass` "/Game/Arkanoid/Core/Blueprints/Bonuses/Positive/BP_DoubleSpeedCarrige.BP_DoubleSpeedCarrige_C" (`KismetMathLibrary.MakeTransform` (`self.SpawnTransformLocationBlock`) (struct) (`self.SpawnTransformScaleExtraBall`)) "Undefined" "OverrideRootScale" null null)
                (elif (`KismetMathLibrary.RandomBoolWithWeight` (`self.RemoveOneBallLiveChance`))
                  (`|SpawnActorFromClass` "/Game/Arkanoid/Core/Blueprints/Bonuses/Negative/BP_RemoveOneBallLife.BP_RemoveOneBallLife_C" (`KismetMathLibrary.MakeTransform` (`self.SpawnTransformLocationBlock`) (struct) (`self.SpawnTransformScaleExtraBall`)) "Undefined" "OverrideRootScale" null null))))))
        (else
          (`self.SetColour` (`self.Lives`)))))))

(fn `SetColour`
  (params (BlockLives :type Integer))
  (switch `int` BlockLives
    (:`1`
      (bind _output_get (set `self.MaterialInstanceColorBlock` (struct :`R` 1.0 :`G` 0.972549 :`A` 1.0)))
      (`MaterialInstanceDynamic.SetVectorParameterValue` (`self.MaterialInstanceBlock`) (`self.MaterialInstanceParameterBlock`) _output_get)
      (return))
    (:`2`
      (bind _output_get_2 (set `self.MaterialInstanceColorBlock` (`KismetMathLibrary.LinearColor_Green`)))
      (`MaterialInstanceDynamic.SetVectorParameterValue` (`self.MaterialInstanceBlock`) (`self.MaterialInstanceParameterBlock`) _output_get_2)
      (return))
    (:`3`
      (bind _output_get_3 (set `self.MaterialInstanceColorBlock` (`KismetMathLibrary.LinearColor_Blue`)))
      (`MaterialInstanceDynamic.SetVectorParameterValue` (`self.MaterialInstanceBlock`) (`self.MaterialInstanceParameterBlock`) _output_get_3)
      (return))
    (:`4`
      (bind _output_get_4 (set `self.MaterialInstanceColorBlock` (`KismetMathLibrary.LinearColor_Red`)))
      (`MaterialInstanceDynamic.SetVectorParameterValue` (`self.MaterialInstanceBlock`) (`self.MaterialInstanceParameterBlock`) _output_get_4)
      (return))))

(fn `UserConstructionScript`)