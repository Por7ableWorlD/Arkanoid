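; BP_Carrige is the player's Arkanoid paddle, which moves sideways and spawns game balls from a limited lives count.
; MoveRight input shifts it by a fixed swept step per axis event, independent of axis magnitude and frame time.
; BeginPlay tints the cube through a dynamic material and calls SpawnBall.
; SpawnBall prints remaining lives, then, if any remain, spawns BP_GameBall, binds its OnDeath event and decrements lives.
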(event `InputAxis|MoveRight`
  (params (AxisValue :type "Float (single-precision)"))
  ;[1 1 1] Right and left carriage movement
  (if (> AxisValue 0.0)
    (`self.K2_AddActorWorldOffset` (4.0 0.0 0.0) true)))

(event `InputAxis|MoveRight`
  (params (AxisValue :type "Float (single-precision)"))
  ;[1 1 1] Right and left carriage movement
  (if (< AxisValue 0.0)
    (`self.K2_AddActorWorldOffset` (-4.0 0.0 0.0) true)))

(event `self.ReceiveBeginPlay`
  (bind _returnvalue (`PrimitiveComponent.CreateDynamicMaterialInstance` (`self.Cube`) 0 null "None"))
  (`MaterialInstanceDynamic.SetVectorParameterValue` _returnvalue "Colour" (struct :`G` 1.0 :`B` 0.890196 :`A` 1.0))
  (`self.SpawnBall`))

(fn `OutputBallLives`
  (locals (TextColor :type "LinearColor Structure" :default (struct :`G` 1.0 :`B` 0.037146 :`A` 1.0)))
  (if (!= (`self.BallLives`) 0)
    (`KismetSystemLibrary.PrintString` (`KismetStringLibrary.Concat_StrStr` "You have " (`KismetStringLibrary.Conv_IntToString` (`self.BallLives`)) " lives") true true (struct :`R` 0.099749 :`G` 1.0 :`A` 1.0) 5.0)
    (else
      (`KismetSystemLibrary.PrintString` (`KismetStringLibrary.Concat_StrStr` "You have " (`KismetStringLibrary.Conv_IntToString` (`self.BallLives`)) " lives") true true (struct :`R` 1.0 :`B` 0.11875 :`A` 1.0) 5.0))))

(fn `SpawnBall`
  (`self.OutputBallLives`)
  (if (> (`self.BallLives`) 0)
    (bind _returnvalue (`|SpawnActorFromClass` "/Game/Arkanoid/Core/Blueprints/BP_GameBall.BP_GameBall_C" (`KismetMathLibrary.MakeTransform` (`SceneComponent.K2_GetComponentLocation` (`self.PlaceBallSpawn`)) (struct) (0.25 0.25 0.25)) "AlwaysSpawn" "OverrideRootScale" null null))
    (bind _output_get (set `self.GameBall` _returnvalue))
    (add `/Game/Arkanoid/Core/Blueprints/BP_GameBall.OnDeath` _output_get (`|CreateDelegate` :!event `SpawnBall`))
    (`/Engine/EditorBlueprintResources/StandardMacros.DecrementInt` (`self.BallLives`)
      (:`  `
        (return)))))

(fn `UserConstructionScript`)