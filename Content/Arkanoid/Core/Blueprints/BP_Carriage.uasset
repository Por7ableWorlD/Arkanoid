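; Player paddle for an Arkanoid game that sweeps sideways on MoveRight input and launches its attached ball on left click.
; SpawnBall creates the ball while lives remain and binds to its OnDeath event; SpawnExtraBall adds extra balls.
; Double and half speed effects scale the move step until a refreshable 10-second timer restores defaults.
; BeginPlay tints the paddle, but assigns the right-move default to itself instead of caching the current step.
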(event `InputAxis|MoveRight`
  (params (AxisValue :type "Float (single-precision)"))
  ;[1 0.06357 0] ПОСМОТЕРТЬ КАК СДЕЛАНО ДВИЖЕНИЕ В ТАНКАХ (ТАМ ЕСТЬ ПРИМЕР ОТКУДА ТО ВЗЯТЫЙ)
  ;;[1 1 1] Right and left carriage movement
  (if (> AxisValue 0.0)
    (`self.K2_AddActorWorldOffset` (`self.MoveRightDeltaLocation`) true)))

(event `InputAxis|MoveRight`
  (params (AxisValue :type "Float (single-precision)"))
  ;[1 0.06357 0] ПОСМОТЕРТЬ КАК СДЕЛАНО ДВИЖЕНИЕ В ТАНКАХ (ТАМ ЕСТЬ ПРИМЕР ОТКУДА ТО ВЗЯТЫЙ)
  ;;[1 1 1] Right and left carriage movement
  (if (< AxisValue 0.0)
    (`self.K2_AddActorWorldOffset` (`self.MoveLeftDeltaLocation`) true)))

(event `self.ReceiveBeginPlay`
  (bind _returnvalue (`PrimitiveComponent.CreateDynamicMaterialInstance` (`self.Carriage`) 0 null "None"))
  (bind _output_get (set `self.MaterialInstance` _returnvalue))
  (`MaterialInstanceDynamic.SetVectorParameterValue` _output_get (`self.MaterialInstanceParameter`) (`self.MaterialInstanceColor`))
  (`self.SpawnBall`)
  (set `self.DefaultMoveLeftDeltaLocation` (`self.MoveLeftDeltaLocation`))
  (set `self.DefaultMoveRightDeltaLocation` (`self.DefaultMoveRightDeltaLocation`)))

(event `self.ReceiveTick`
  (params (DeltaSeconds :type "Float (single-precision)"))
  (bind _timerdoublespeed (`self.TimerDoubleSpeed`))
  (bind _returnvalue (`KismetSystemLibrary.K2_GetTimerRemainingTimeHandle` _timerdoublespeed))
  ;[1 1 1] Вывод количества секунд (до милисекунд) до окончания действия двойной скорости каретки
  (if (and (`KismetSystemLibrary.K2_IsValidTimerHandle` _timerdoublespeed) (> _returnvalue 0.0))
    (`KismetSystemLibrary.PrintString` (`KismetStringLibrary.Conv_DoubleToString` _returnvalue) true true (struct :`R` 1.0 :`B` 0.940979 :`A` 1.0) 0.0)))

(event `Key|LeftMouseButton`
  (params (Key :type "Key Structure"))
  (:`Pressed`
    (set `/Game/Arkanoid/Core/Blueprints/BP_GameBall.IsBallStart` true (`self.GameBall`))
    (`self.K2_DetachFromActor` (`self.GameBall`) "KeepWorld" "KeepWorld" "KeepWorld")))

(fn `DecreaseBallLives`
  (`/Engine/EditorBlueprintResources/StandardMacros.DecrementInt` (`self.BallLives`)
    (:`  `
      (return))))

(fn `GetGameBall`
  (returns (GameBall :type "/Game/Arkanoid/Core/Blueprints/BP_GameBall Object Reference"))
  (return (`self.GameBall`)))

(fn `GetInfoDoubleDownSpeed`
  (returns (DoubleDownSpeed :type Boolean))
  (return (`self.IsDoubleDownSpeed`)))

(fn `GetInfoDoubleUpSpeed`
  (returns (DoubleUpSpeed :type Boolean))
  (return (`self.IsDoubleUpSpeed`)))

(fn `OutputBallLives`
  (locals (TextColor :type "LinearColor Structure" :default (struct :`G` 1.0 :`B` 0.037146 :`A` 1.0)))
  (if (!= (`self.BallLives`) 0)
    (`KismetSystemLibrary.PrintString` (`KismetStringLibrary.Concat_StrStr` "You have " (`KismetStringLibrary.Conv_IntToString` (`self.BallLives`)) " lives") true true (struct :`R` 0.099749 :`G` 1.0 :`A` 1.0) 5.0)
    (else
      (`KismetSystemLibrary.PrintString` "YOU LOSE!" true true (struct :`R` 1.0 :`B` 0.11875 :`A` 1.0) 5.0)))
  (return))

(fn `SetDefaultSpeed`
  (bind _doubleupspeed (`self.GetInfoDoubleUpSpeed`))
  (if _doubleupspeed
    (set `self.IsDoubleUpSpeed` false)
    (set `self.MoveLeftDeltaLocation` (`self.DefaultMoveLeftDeltaLocation`) :!label _label)
    (set `self.MoveRightDeltaLocation` (`self.DefaultMoveRightDeltaLocation`))
    (`KismetSystemLibrary.K2_ClearAndInvalidateTimerHandle` (`self.TimerDoubleSpeed`))
    (else
      (bind _doubledownspeed (`self.GetInfoDoubleDownSpeed`))
      (if _doubledownspeed
        (set `self.IsDoubleDownSpeed` false)
        (goto _label)
        (else
          _))))
  (return))

(fn `SetDoubleDownSpeed`
  (add `/Game/Arkanoid/Core/Blueprints/BP_GameBall.OnDeath` (`self.GameBall`) (`|CreateDelegate` :!event `SetDefaultSpeed`))
  (bind _doubledownspeed (`self.GetInfoDoubleDownSpeed`))
  (if _doubledownspeed
    (bind _returnvalue (`KismetSystemLibrary.K2_SetTimer` null "SetDefaultSpeed" 10.0))
    (set `self.TimerDoubleSpeed` _returnvalue)
    (else
      (set `self.MoveLeftDeltaLocation` (`KismetMathLibrary.MakeVector` (/ (.x (`self.MoveLeftDeltaLocation`)) 2.0)))
      (set `self.MoveRightDeltaLocation` (`KismetMathLibrary.MakeVector` (/ (.x (`self.MoveRightDeltaLocation`)) 2.0)))
      (set `self.IsDoubleDownSpeed` true)
      (bind _returnvalue_2 (`KismetSystemLibrary.K2_SetTimer` null "SetDefaultSpeed" 10.0))
      (set `self.TimerDoubleSpeed` _returnvalue_2)))
  (return))

(fn `SetDoubleUpSpeed`
  (add `/Game/Arkanoid/Core/Blueprints/BP_GameBall.OnDeath` (`self.GameBall`) (`|CreateDelegate` :!event `SetDefaultSpeed`))
  (bind _doubleupspeed (`self.GetInfoDoubleUpSpeed`))
  (if _doubleupspeed
    (bind _returnvalue (`KismetSystemLibrary.K2_SetTimer` null "SetDefaultSpeed" 10.0))
    (set `self.TimerDoubleSpeed` _returnvalue)
    (else
      (set `self.MoveLeftDeltaLocation` (`KismetMathLibrary.MakeVector` (* (.x (`self.MoveLeftDeltaLocation`)) 2.0)))
      (set `self.MoveRightDeltaLocation` (`KismetMathLibrary.MakeVector` (* (.x (`self.MoveRightDeltaLocation`)) 2.0)))
      (set `self.IsDoubleUpSpeed` true)
      (bind _returnvalue_2 (`KismetSystemLibrary.K2_SetTimer` null "SetDefaultSpeed" 10.0))
      (set `self.TimerDoubleSpeed` _returnvalue_2)))
  (return))

(fn `SpawnBall`
  (`self.OutputBallLives`)
  (if (> (`self.BallLives`) 0)
    (bind _returnvalue (`|SpawnActorFromClass` "/Game/Arkanoid/Core/Blueprints/BP_GameBall.BP_GameBall_C" (`KismetMathLibrary.MakeTransform` (`SceneComponent.K2_GetComponentLocation` (`self.PlaceBallSpawn`)) (struct) (`self.SpawnTransformScaleBall`)) "AlwaysSpawn" "OverrideRootScale" null null))
    (bind _output_get (set `self.GameBall` _returnvalue))
    (`self.K2_AttachToComponent` _output_get (`self.PlaceBallSpawn`) "None" "KeepWorld" "KeepWorld" "KeepWorld" true)
    (add `/Game/Arkanoid/Core/Blueprints/BP_GameBall.OnDeath` (`self.GameBall`) (`|CreateDelegate` :!event `DecreaseBallLives`))
    (add `/Game/Arkanoid/Core/Blueprints/BP_GameBall.OnDeath` (`self.GameBall`) (`|CreateDelegate` :!event `SpawnBall`))
    (return)))

(fn `SpawnExtraBall`
  (if (`/Game/Arkanoid/Core/Blueprints/BP_GameBall.IsBallStart` (`self.GameBall`))
    (bind _returnvalue (`|SpawnActorFromClass` "/Game/Arkanoid/Core/Blueprints/BP_ExtraBall.BP_ExtraBall_C" (`KismetMathLibrary.MakeTransform` (`SceneComponent.K2_GetComponentLocation` (`self.PlaceBallSpawn`)) (struct) (`self.SpawnTransformScaleBall`)) "AlwaysSpawn" "OverrideRootScale" null null))
    (bind _output_get (set `self.ExtraBall` _returnvalue))
    (`/Game/Arkanoid/Core/Blueprints/BP_ExtraBall.SetDirection` _output_get)
    (return)
    (elif (`KismetMathLibrary.RandomBoolWithWeight` 0.5)
      (`|SpawnActorFromClass` "/Game/Arkanoid/Core/Blueprints/BP_ExtraBall.BP_ExtraBall_C" (`KismetMathLibrary.MakeTransform` (`KismetMathLibrary.MakeVector` (+ (.x (`SceneComponent.K2_GetComponentLocation` (`self.PlaceBallSpawn`))) 30.0) (.y (`SceneComponent.K2_GetComponentLocation` (`self.PlaceBallSpawn`))) (.z (`SceneComponent.K2_GetComponentLocation` (`self.PlaceBallSpawn`)))) (struct) (`self.SpawnTransformScaleBall`)) "AlwaysSpawn" "OverrideRootScale" null null)
      (else
        (`|SpawnActorFromClass` "/Game/Arkanoid/Core/Blueprints/BP_ExtraBall.BP_ExtraBall_C" (`KismetMathLibrary.MakeTransform` (`KismetMathLibrary.MakeVector` (- (.x (`SceneComponent.K2_GetComponentLocation` (`self.PlaceBallSpawn`))) 30.0) (.y (`SceneComponent.K2_GetComponentLocation` (`self.PlaceBallSpawn`))) (.z (`SceneComponent.K2_GetComponentLocation` (`self.PlaceBallSpawn`)))) (struct) (`self.SpawnTransformScaleBall`)) "AlwaysSpawn" "OverrideRootScale" null null)))))

(fn `UserConstructionScript`)