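; BP_DoubleDamageBall is a positive bonus in the Arkanoid game that turns on double damage for the ball.
; On overlap it runs the parent handler, then casts the other actor to BP_Carriage.
; If that carriage's GameBall lacks IsDoubleDamage, it sets the flag and prints an on-screen message.
; Nothing in this Blueprint clears the flag.
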(event `self.ReceiveActorBeginOverlap`
  (params (OtherActor :type "Actor Object Reference"))
  (`parent.ReceiveActorBeginOverlap` OtherActor)
  (bind _asbp_carriage (cast `/Game/Arkanoid/Core/Blueprints/BP_Carriage` OtherActor))
  (bind _gameball (`/Game/Arkanoid/Core/Blueprints/BP_Carriage.GameBall` _asbp_carriage))
  (if (not (`/Game/Arkanoid/Core/Blueprints/BP_GameBall.IsDoubleDamage` _gameball))
    (set `/Game/Arkanoid/Core/Blueprints/BP_GameBall.IsDoubleDamage` true _gameball)
    (`KismetSystemLibrary.PrintString` "DoubleDamage ON" true true (struct :`R` 1.0 :`B` 0.127135 :`A` 1.0) 5.0)))

(fn `UserConstructionScript`
  (`parent.UserConstructionScript`))