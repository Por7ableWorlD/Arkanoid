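; BP_ExtraBall is a positive bonus pickup in an Arkanoid game that grants the player an additional ball.
; When it overlaps BP_Carriage, it runs the parent overlap logic, then spawns a BP_GameBall at the carriage's ball spawn point using the carriage's ball scale.
; The new ball's dynamic material color parameter is set to the extra-ball color to tint it.
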(event `self.ReceiveBeginPlay`
  (`parent.ReceiveBeginPlay`))

(event `self.ReceiveActorBeginOverlap`
  (params (OtherActor :type "Actor Object Reference"))
  (`parent.ReceiveActorBeginOverlap` OtherActor)
  (bind _asbp_carriage (cast `/Game/Arkanoid/Core/Blueprints/BP_Carriage` OtherActor))
  (bind _returnvalue (`|SpawnActorFromClass` "/Game/Arkanoid/Core/Blueprints/BP_GameBall.BP_GameBall_C" (`KismetMathLibrary.MakeTransform` (`SceneComponent.K2_GetComponentLocation` (`/Game/Arkanoid/Core/Blueprints/BP_Carriage.PlaceBallSpawn` _asbp_carriage)) (struct) (`/Game/Arkanoid/Core/Blueprints/BP_Carriage.SpawnTransformScaleBall` _asbp_carriage)) "Undefined" "OverrideRootScale" null null))
  (bind _output_get (set `/Game/Arkanoid/Core/Blueprints/BP_GameBall.MaterialInstanceColorBall` (`self.MaterialInstanceColorExtraBall`) _returnvalue))
  (`MaterialInstanceDynamic.SetVectorParameterValue` (`/Game/Arkanoid/Core/Blueprints/BP_GameBall.MaterialInstanceBall` _returnvalue) (`/Game/Arkanoid/Core/Blueprints/BP_GameBall.MaterialInstanceParameterBall` _returnvalue) _output_get))

(fn `UserConstructionScript`
  (`parent.UserConstructionScript`))