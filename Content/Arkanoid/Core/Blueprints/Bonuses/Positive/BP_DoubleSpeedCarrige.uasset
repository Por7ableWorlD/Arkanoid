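; BP_DoubleSpeedCarrige is a positive Arkanoid bonus that doubles the carriage's movement speed.
; On overlap it runs the parent handler, then casts the other actor to BP_Carriage.
; It doubles the X of the left and right move deltas, zeroing Y and Z.
; The carriage's IsDoubleCarriageSpeed flag prevents stacking, and this Blueprint never reverts the boost.
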(event `self.ReceiveActorBeginOverlap`
  (params (OtherActor :type "Actor Object Reference"))
  (`parent.ReceiveActorBeginOverlap` OtherActor)
  (bind _asbp_carriage (cast `/Game/Arkanoid/Core/Blueprints/BP_Carriage` OtherActor))
  (if (not (`/Game/Arkanoid/Core/Blueprints/BP_Carriage.IsDoubleCarriageSpeed` _asbp_carriage))
    (bind _moveleftdeltalocation_x (`KismetMathLibrary.BreakVector` (`/Game/Arkanoid/Core/Blueprints/BP_Carriage.MoveLeftDeltaLocation` _asbp_carriage)))
    (set `/Game/Arkanoid/Core/Blueprints/BP_Carriage.MoveLeftDeltaLocation` (`KismetMathLibrary.MakeVector` (* _moveleftdeltalocation_x 2.0)) _asbp_carriage)
    (bind _moverightdeltalocation_x (`KismetMathLibrary.BreakVector` (`/Game/Arkanoid/Core/Blueprints/BP_Carriage.MoveRightDeltaLocation` _asbp_carriage)))
    (set `/Game/Arkanoid/Core/Blueprints/BP_Carriage.MoveRightDeltaLocation` (`KismetMathLibrary.MakeVector` (* _moverightdeltalocation_x 2.0)) _asbp_carriage)
    (set `/Game/Arkanoid/Core/Blueprints/BP_Carriage.IsDoubleCarriageSpeed` true _asbp_carriage)))

(fn `UserConstructionScript`
  (`parent.UserConstructionScript`))