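; BP_BaseBonus is the base actor for bonus pickups in the Arkanoid game.
; On BeginPlay it creates a dynamic material on the Bonus component and tints it with a configurable color parameter.
; Each tick it moves along its Direction at Speed with a swept offset, and it destroys itself when it overlaps a KillZVolume.
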(event `self.ReceiveBeginPlay`
  (bind _returnvalue (`PrimitiveComponent.CreateDynamicMaterialInstance` (`self.Bonus`) 0 null "None"))
  (bind _output_get (set `self.MaterialInstanceBonus` _returnvalue))
  (`MaterialInstanceDynamic.SetVectorParameterValue` _output_get (`self.MaterialInstanceParameterBonus`) (`self.MaterialInstanceColorBonus`)))

(event `self.ReceiveActorBeginOverlap`
  (params (OtherActor :type "Actor Object Reference"))
  (cast `KillZVolume` OtherActor)
  (`self.K2_DestroyActor`))

(event `self.ReceiveTick`
  (params (DeltaSeconds :type "Float (single-precision)"))
  (`self.K2_AddActorWorldOffset` (* (* (`self.Direction`) (`self.Speed`)) DeltaSeconds) true))

(fn `UserConstructionScript`)