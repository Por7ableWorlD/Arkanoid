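; BP_ExtraBall is an additional ball actor for the Arkanoid game, which moves on its own and bounces off whatever it hits.
; Each tick it sweeps the ball component along Direction times Speed, reflecting Direction on a blocking hit using only the normal's X and Y to stay in the scene.
; It tints itself through a dynamic material instance on BeginPlay and destroys itself upon overlapping a KillZVolume.
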(event `self.ReceiveBeginPlay`
  (bind _returnvalue (`PrimitiveComponent.CreateDynamicMaterialInstance` (`self.ExtraBall`) 0 null "None"))
  (bind _output_get (set `self.MaterialInstance` _returnvalue))
  (`MaterialInstanceDynamic.SetVectorParameterValue` _output_get (`self.MaterialInstanceParameter`) (`self.MaterialInstanceColor`)))

(event `self.ReceiveActorBeginOverlap`
  (params (OtherActor :type "Actor Object Reference"))
  (cast `KillZVolume` OtherActor)
  (`self.K2_DestroyActor` self))

(event `self.ReceiveTick`
  (params (DeltaSeconds :type "Float (single-precision)"))
  (bind _sweephitresult (`SceneComponent.K2_AddLocalOffset` (`self.ExtraBall`) (* (* (`self.Direction`) (`self.Speed`)) DeltaSeconds) true false))
  (bind (_bblockinghit _binitialoverlap _time _distance _location _impactpoint _normal) (`GameplayStatics.BreakHitResult` _sweephitresult))
  (if _bblockinghit
    (set `self.Direction` (`KismetMathLibrary.GetReflectionVector` (`self.Direction`) (`KismetMathLibrary.MakeVector` (.x _normal) (.y _normal))))))

(fn `UserConstructionScript`)