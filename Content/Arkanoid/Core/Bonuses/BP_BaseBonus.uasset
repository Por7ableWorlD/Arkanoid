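; Base bonus pickup actor for an Arkanoid game, moving along a set direction until destroyed.
; BeginPlay tints the Bonus component through a dynamic material instance and caches the starting speed; Tick applies a swept, frame-rate-independent move.
; Overlapping a kill-Z volume or the carriage destroys it, with no effect applied here.
; StopBonus zeroes the speed and RunBonus restores the cached value, pausing and resuming movement.
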(event `self.ReceiveBeginPlay`
  (bind _returnvalue (`PrimitiveComponent.CreateDynamicMaterialInstance` (`self.Bonus`) 0 null "None"))
  (bind _output_get (set `self.MaterialInstance` _returnvalue))
  (`MaterialInstanceDynamic.SetVectorParameterValue` _output_get (`self.MaterialInstanceParameter`) (`self.MaterialInstanceColor`))
  (set `self.DefaultSpeed` (`self.Speed`)))

(event `self.ReceiveActorBeginOverlap`
  (params (OtherActor :type "Actor Object Reference"))
  (cast `KillZVolume` OtherActor
    (:`then`
      (`self.K2_DestroyActor`))
    (:`CastFailed`
      (cast `/Game/Arkanoid/Core/GameObjects/BP_Carriage` OtherActor)
      (`self.K2_DestroyActor`))))

(event `self.ReceiveTick`
  (params (DeltaSeconds :type "Float (single-precision)"))
  (`self.K2_AddActorWorldOffset` (* (* (`self.Direction`) (`self.Speed`)) DeltaSeconds) true))

(fn `RunBonus`
  (`self.SetDefaultSpeed` self)
  (return))

(fn `SetDefaultSpeed`
  (set `self.Speed` (`self.DefaultSpeed`))
  (return))

(fn `StopBonus`
  (set `self.Speed` 0.0)
  (return))

(fn `UserConstructionScript`)