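; Player paddle of the Arkanoid game that also runs the match: ball lives, block count, pause and win/lose screens.
; Axis input moves it with swept offsets, and a click launches the attached ball spawned by SpawnBall.
; Bound ball and block events support life and win tracking, feeding the HUD widget.
; Bonus functions add extra balls or temporarily double or halve speed, while pause manually stops balls, bonuses and paddle.
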(event `InputAxis|MoveRight`
  (params (AxisValue :type "Float (single-precision)"))
  ;[1 0.06357 0] ПОСМОТЕРТЬ КАК СДЕЛАНО ДВИЖЕНИЕ В ТАНКАХ (ТАМ ЕСТЬ ПРИМЕР ОТКУДА ТО ВЗЯТЫЙ)
  ;;[1 1 1] Right and left carriage movement
  (if (> AxisValue 0.0)
    (`self.K2_AddActorWorldOffset` (`self.MoveRightDeltaLocation`) true)))

(event `InputAxis|MoveRight`
  (params (AxisValue :type "Float (single-precision)"))
  ;[1 0.06357 0] ПОСМОТЕРТЬ КАК СДЕЛАНО ДВИЖЕНИЕ В ТАНКАХ (ТАМ ЕСТЬ ПРИМЕР ОТКУДА ТО ВЗЯТЫЙ)
  ;;[1 1 1] Right and left carriage movement
  (if (< AxisValue 0.0)
    (`self.K2_AddActorWorldOffset` (`self.MoveLeftDeltaLocation`) true)))

(event `self.ReceiveBeginPlay`
  (bind _returnvalue (`PrimitiveComponent.CreateDynamicMaterialInstance` (`self.Carriage`) 0 null "None"))
  (bind _output_get (set `self.MaterialInstance` _returnvalue))
  (`MaterialInstanceDynamic.SetVectorParameterValue` _output_get (`self.MaterialInstanceParameter`) (`self.MaterialInstanceColor`))
  (`self.SpawnBall`)
  (set `self.DefaultMoveLeftDeltaLocation` (`self.MoveLeftDeltaLocation`))
  (set `self.DefaultMoveRightDeltaLocation` (`self.DefaultMoveRightDeltaLocation`))
  (bind _outactors (`GameplayStatics.GetAllActorsOfClass` "/Game/Arkanoid/Core/Blocks/BP_BaseBlock.BP_BaseBlock_C"))
  (bind _output_get_2 (set `self.BaseBlocks` _outactors))
  (set `self.AmountBlocks` (`KismetArrayLibrary.Array_Length` _output_get_2))
  (for _array_element (`self.BaseBlocks`)
    (add `/Game/Arkanoid/Core/Blocks/BP_BaseBlock.OnDestroy` _array_element (`|CreateDelegate` :!event `CheckWinGame`))
    (bind _returnvalue_2 (`|CreateWidget` "/Game/Arkanoid/Core/UI/Screens/WBP_GameScreen.WBP_GameScreen_C" (`GameplayStatics.GetPlayerController` 0)))
    (bind _output_get_3 (set `self.GameScreenWidget` _returnvalue_2))
    (`/Game/Arkanoid/Core/UI/Screens/WBP_GameScreen.SetLives` _output_get_3 (`self.BallLives`))
    (`UserWidget.AddToViewport` (`self.GameScreenWidget`) 0)
    (`WidgetBlueprintLibrary.SetInputMode_GameOnly` (`GameplayStatics.GetPlayerController` 0))))

(event `self.ReceiveTick`
  (params (DeltaSeconds :type "Float (single-precision)"))
  (bind _timerdoublespeed (`self.TimerDoubleSpeed`))
  (bind _returnvalue (`KismetSystemLibrary.K2_GetTimerRemainingTimeHandle` _timerdoublespeed))
  (if (and (`KismetSystemLibrary.K2_IsValidTimerHandle` _timerdoublespeed) (> _returnvalue 0.0))
    (`/Game/Arkanoid/Core/UI/Screens/WBP_GameScreen.SetCarriageSpeedDownTimer` (`self.GameScreenWidget`) (/ (`KismetMathLibrary.Conv_IntToDouble` (`KismetMathLibrary.Round` (* 10 _returnvalue))) 10.0))))

(event `Key|LeftMouseButton`
  (params (Key :type "Key Structure"))
  (:`Pressed`
    (bind _isrun (`/Game/Arkanoid/Core/GameObjects/BP_GameBall.GetInfoBallRunning` (`self.GameBall`)))
    (if (not _isrun)
      (`/Game/Arkanoid/Core/GameObjects/BP_GameBall.RunBall` (`self.GameBall`))
      (`self.K2_DetachFromActor` (`self.GameBall`) "KeepWorld" "KeepWorld" "KeepWorld")
      (`PrimitiveComponent.SetCollisionEnabled` (`/Game/Arkanoid/Core/GameObjects/BP_GameBall.Ball` (`self.GameBall`)) "QueryAndPhysics"))))

(event `Key|Escape`
  (params (Key :type "Key Structure"))
  (bind _returnvalue (`GameplayStatics.GetPlayerController` 0))
  (:`Pressed`
    (`self.PauseGame`)
    (`WidgetBlueprintLibrary.SetInputMode_UIOnlyEx` (`GameplayStatics.GetPlayerController` 0) null)
    (set `PlayerController.bShowMouseCursor` true _returnvalue)
    (bind _returnvalue_2 (`|CreateWidget` "/Game/Arkanoid/Core/UI/Menu/Pause/WBP_PauseMenu.WBP_PauseMenu_C" _returnvalue))
    (bind _output_get (set `self.PauseMenuWidget` _returnvalue_2))
    (`UserWidget.AddToViewport` _output_get 0)
    (add `/Game/Arkanoid/Core/UI/Menu/Pause/WBP_PauseMenu.OnResumePressed` (`self.PauseMenuWidget`) (`|CreateDelegate` :!event `ResumeGame`))))

(fn `CheckWinGame`
  (bind _updateamountblocks (`self.DecreaseAmountBlocks`))
  (if (<= _updateamountblocks 0)
    (bind _returnvalue (`KismetSystemLibrary.K2_SetTimer` null "StopGame" 0.05))
    (set `self.TimerShowWidgets` _returnvalue))
  (return))

(fn `DecreaseAmountBlocks`
  (returns (UpdateAmountBlocks :type Integer))
  (bind _result (`/Engine/EditorBlueprintResources/StandardMacros.DecrementInt` (`self.AmountBlocks`))
    (:`  `
      (return _result))))

(fn `DecreaseBallLives`
  (bind _result (`/Engine/EditorBlueprintResources/StandardMacros.DecrementInt` (`self.BallLives`))
    (:`  `
      (`/Game/Arkanoid/Core/UI/Screens/WBP_GameScreen.SetLives` (`self.GameScreenWidget`) _result)
      (return))))

(fn `DeletePlayableActors`
  (bind _outactors (`GameplayStatics.GetAllActorsOfClass` "/Game/Arkanoid/Core/GameObjects/BP_ExtraBall.BP_ExtraBall_C"))
  (for _array_element _outactors
    (`self.K2_DestroyActor` _array_element))
  (bind _outactors_2 (`GameplayStatics.GetAllActorsOfClass` "/Game/Arkanoid/Core/Bonuses/BP_BaseBonus.BP_BaseBonus_C"))
  (for _array_element_2 _outactors_2
    (`self.K2_DestroyActor` _array_element_2))
  (return))

(fn `GetBallLives`
  (returns (BallLives :type Integer))
  (return (`self.BallLives`)))

(fn `GetGameBall`
  (returns (GameBall :type "/Game/Arkanoid/Core/GameObjects/BP_GameBall Object Reference"))
  (return (`self.GameBall`)))

(fn `GetInfoDoubleDownSpeed`
  (returns (DoubleDownSpeed :type Boolean))
  (return (`self.IsDoubleDownSpeed`)))

(fn `GetInfoDoubleUpSpeed`
  (returns (DoubleUpSpeed :type Boolean))
  (return (`self.IsDoubleUpSpeed`)))

(fn `IncreaseBallLives`
  (bind _result (`/Engine/EditorBlueprintResources/StandardMacros.IncrementInt` (`self.BallLives`))
    (:`  `
      (`/Game/Arkanoid/Core/UI/Screens/WBP_GameScreen.SetLives` (`self.GameScreenWidget`) _result)
      (return))))

(fn `PauseGame`
  (`/Game/Arkanoid/Core/GameObjects/BP_GameBall.StopBall` (`self.GameBall`))
  (`self.StopCarriage` self)
  (bind _outactors (`GameplayStatics.GetAllActorsOfClass` "/Game/Arkanoid/Core/GameObjects/BP_ExtraBall.BP_ExtraBall_C"))
  (for _array_element _outactors
    (`/Game/Arkanoid/Core/GameObjects/BP_ExtraBall.StopBall` _array_element))
  (bind _outactors_2 (`GameplayStatics.GetAllActorsOfClass` "/Game/Arkanoid/Core/Bonuses/BP_BaseBonus.BP_BaseBonus_C"))
  (for _array_element_2 _outactors_2
    (`/Game/Arkanoid/Core/Bonuses/BP_BaseBonus.StopBonus` _array_element_2))
  (return))

(fn `ResumeGame`
  (`/Engine/EditorBlueprintResources/StandardMacros.IsValid` (`self.GameBall`)
    (:`Is Valid`
      (bind _isrun (`/Game/Arkanoid/Core/GameObjects/BP_GameBall.GetInfoBallRunning` (`self.GameBall`)))
      (if (not _isrun)
        (`/Game/Arkanoid/Core/GameObjects/BP_GameBall.RunBall` (`self.GameBall`))
        (`self.RunCarriage` self)
        (bind _outactors (`GameplayStatics.GetAllActorsOfClass` "/Game/Arkanoid/Core/GameObjects/BP_ExtraBall.BP_ExtraBall_C"))
        (for _array_element _outactors
          (`/Game/Arkanoid/Core/GameObjects/BP_ExtraBall.RunBall` _array_element))
        (bind _outactors_2 (`GameplayStatics.GetAllActorsOfClass` "/Game/Arkanoid/Core/Bonuses/BP_BaseBonus.BP_BaseBonus_C"))
        (for _array_element_2 _outactors_2
          (`/Game/Arkanoid/Core/Bonuses/BP_BaseBonus.RunBonus` _array_element_2))))
    (:`Is Not Valid`
      _))
  (return))

(fn `RunCarriage`
  (bind _doubleupspeed (`self.GetInfoDoubleUpSpeed`))
  (if _doubleupspeed
    (`self.SetDoubleUpSpeed`)
    (else
      (bind _doubledownspeed (`self.GetInfoDoubleDownSpeed`))
      (if _doubledownspeed
        (`self.SetDoubleDownSpeed`)
        (else
          (`self.SetDefaultSpeed`)))))
  (return))

(fn `RunLoseWidget`
  (bind _returnvalue (`|CreateWidget` "/Game/Arkanoid/Core/UI/Screens/WBP_LoseScreen.WBP_LoseScreen_C" (`GameplayStatics.GetPlayerController` 0)))
  (`UserWidget.AddToViewport` _returnvalue 0)
  (if (`KismetSystemLibrary.K2_IsValidTimerHandle` (`self.TimerStopGame`))
    (`KismetSystemLibrary.K2_ClearAndInvalidateTimerHandle` (`self.TimerStopGame`)))
  (return))

(fn `RunWinWidget`
  (bind _returnvalue (`|CreateWidget` "/Game/Arkanoid/Core/UI/Screens/WBP_WinScreen.WBP_WinScreen_C" (`GameplayStatics.GetPlayerController` 0)))
  (`UserWidget.AddToViewport` _returnvalue 0)
  (if (`KismetSystemLibrary.K2_IsValidTimerHandle` (`self.TimerStopGame`))
    (`KismetSystemLibrary.K2_ClearAndInvalidateTimerHandle` (`self.TimerStopGame`)))
  (return))

(fn `SetBallDoubleDamageCountToWidget`
  (bind _doubledamagecount (`/Game/Arkanoid/Core/GameObjects/BP_GameBall.GetDoubleDamageCount` (`self.GameBall`)))
  (`/Game/Arkanoid/Core/UI/Screens/WBP_GameScreen.SetDoubleDamage` (`self.GameScreenWidget`) _doubledamagecount)
  (add `/Game/Arkanoid/Core/GameObjects/BP_GameBall.OnDoubleDamageCountChanged` (`self.GameBall`) (`|CreateDelegate` :!event `SetBallDoubleDamageCountToWidget`))
  (return))

(fn `SetDefaultSpeed`
  (bind _doubleupspeed (`self.GetInfoDoubleUpSpeed`))
  (if _doubleupspeed
    (set `self.IsDoubleUpSpeed` false)
    (else
      (bind _doubledownspeed (`self.GetInfoDoubleDownSpeed`))
      (if _doubledownspeed
        (set `self.IsDoubleDownSpeed` false))))
  (set `self.MoveLeftDeltaLocation` (`self.DefaultMoveLeftDeltaLocation`))
  (set `self.MoveRightDeltaLocation` (`self.DefaultMoveRightDeltaLocation`))
  (`KismetSystemLibrary.K2_ClearAndInvalidateTimerHandle` (`self.TimerDoubleSpeed`))
  (`/Game/Arkanoid/Core/UI/Screens/WBP_GameScreen.SetCarriageSpeedDownTimer` (`self.GameScreenWidget`) 0.0)
  (return))

(fn `SetDoubleDownSpeed`
  (add `/Game/Arkanoid/Core/GameObjects/BP_GameBall.OnDeath` (`self.GameBall`) (`|CreateDelegate` :!event `SetDefaultSpeed`))
  (bind _doubledownspeed (`self.GetInfoDoubleDownSpeed`))
  (if _doubledownspeed
    (bind _returnvalue (`KismetSystemLibrary.K2_SetTimer` null "SetDefaultSpeed" 10.0))
    (set `self.TimerDoubleSpeed` _returnvalue)
    (else
      (`self.SetDefaultSpeed`)
      (set `self.MoveLeftDeltaLocation` (`KismetMathLibrary.MakeVector` (/ (.x (`self.MoveLeftDeltaLocation`)) 2.0)))
      (set `self.MoveRightDeltaLocation` (`KismetMathLibrary.MakeVector` (/ (.x (`self.MoveRightDeltaLocation`)) 2.0)))
      (set `self.IsDoubleDownSpeed` true)
      (bind _returnvalue_2 (`KismetSystemLibrary.K2_SetTimer` null "SetDefaultSpeed" 10.0))
      (set `self.TimerDoubleSpeed` _returnvalue_2)))
  (return))

(fn `SetDoubleUpSpeed`
  (add `/Game/Arkanoid/Core/GameObjects/BP_GameBall.OnDeath` (`self.GameBall`) (`|CreateDelegate` :!event `SetDefaultSpeed`))
  (bind _doubleupspeed (`self.GetInfoDoubleUpSpeed`))
  (if _doubleupspeed
    (bind _returnvalue (`KismetSystemLibrary.K2_SetTimer` null "SetDefaultSpeed" 10.0))
    (set `self.TimerDoubleSpeed` _returnvalue)
    (else
      (`self.SetDefaultSpeed`)
      (set `self.MoveLeftDeltaLocation` (`KismetMathLibrary.MakeVector` (* (.x (`self.MoveLeftDeltaLocation`)) 2.0)))
      (set `self.MoveRightDeltaLocation` (`KismetMathLibrary.MakeVector` (* (.x (`self.MoveRightDeltaLocation`)) 2.0)))
      (set `self.IsDoubleUpSpeed` true)
      (bind _returnvalue_2 (`KismetSystemLibrary.K2_SetTimer` null "SetDefaultSpeed" 10.0))
      (set `self.TimerDoubleSpeed` _returnvalue_2)))
  (return))

(fn `SpawnBall`
  (if (> (`self.BallLives`) 0)
    (bind _returnvalue (`|SpawnActorFromClass` "/Game/Arkanoid/Core/GameObjects/BP_GameBall.BP_GameBall_C" (`KismetMathLibrary.MakeTransform` (`SceneComponent.K2_GetComponentLocation` (`self.PlaceBallSpawn`)) (struct) (`self.SpawnScaleBall`)) "AlwaysSpawn" "OverrideRootScale" null null))
    (bind _output_get (set `self.GameBall` _returnvalue))
    (`self.K2_AttachToComponent` _output_get (`self.PlaceBallSpawn`) "None" "KeepWorld" "KeepWorld" "KeepWorld" true)
    (`PrimitiveComponent.SetCollisionEnabled` (`/Game/Arkanoid/Core/GameObjects/BP_GameBall.Ball` (`self.GameBall`)) "NoCollision")
    (add `/Game/Arkanoid/Core/GameObjects/BP_GameBall.OnDeath` (`self.GameBall`) (`|CreateDelegate` :!event `DecreaseBallLives`))
    (add `/Game/Arkanoid/Core/GameObjects/BP_GameBall.OnDeath` (`self.GameBall`) (`|CreateDelegate` :!event `SpawnBall`))
    (add `/Game/Arkanoid/Core/GameObjects/BP_GameBall.OnDeath` (`self.GameBall`) (`|CreateDelegate` :!event `DeletePlayableActors`))
    (add `/Game/Arkanoid/Core/GameObjects/BP_GameBall.OnDoubleDamageCountChanged` (`self.GameBall`) (`|CreateDelegate` :!event `SetBallDoubleDamageCountToWidget`))
    (else
      (`self.StopGame`)))
  (return))

(fn `SpawnExtraBall`
  (bind _gameball (`self.GameBall`))
  (`/Engine/EditorBlueprintResources/StandardMacros.IsValid` _gameball
    (:`Is Valid`
      (bind _isrun (`/Game/Arkanoid/Core/GameObjects/BP_GameBall.GetInfoBallRunning` _gameball))
      (if _isrun
        (bind _returnvalue (`|SpawnActorFromClass` "/Game/Arkanoid/Core/GameObjects/BP_ExtraBall.BP_ExtraBall_C" (`KismetMathLibrary.MakeTransform` (`SceneComponent.K2_GetComponentLocation` (`self.PlaceBallSpawn`)) (struct) (`self.SpawnScaleBall`)) "AlwaysSpawn" "OverrideRootScale" null null))
        (bind _output_get (set `self.ExtraBall` _returnvalue))
        (`/Game/Arkanoid/Core/GameObjects/BP_ExtraBall.SetDirection` _output_get)
        (elif (`KismetMathLibrary.RandomBoolWithWeight` 0.5)
          (`|SpawnActorFromClass` "/Game/Arkanoid/Core/GameObjects/BP_ExtraBall.BP_ExtraBall_C" (`KismetMathLibrary.MakeTransform` (`KismetMathLibrary.MakeVector` (+ (.x (`SceneComponent.K2_GetComponentLocation` (`self.PlaceBallSpawn`))) 30.0) (.y (`SceneComponent.K2_GetComponentLocation` (`self.PlaceBallSpawn`))) (.z (`SceneComponent.K2_GetComponentLocation` (`self.PlaceBallSpawn`)))) (struct) (`self.SpawnScaleBall`)) "AlwaysSpawn" "OverrideRootScale" null null)
          (else
            (`|SpawnActorFromClass` "/Game/Arkanoid/Core/GameObjects/BP_ExtraBall.BP_ExtraBall_C" (`KismetMathLibrary.MakeTransform` (`KismetMathLibrary.MakeVector` (- (.x (`SceneComponent.K2_GetComponentLocation` (`self.PlaceBallSpawn`))) 30.0) (.y (`SceneComponent.K2_GetComponentLocation` (`self.PlaceBallSpawn`))) (.z (`SceneComponent.K2_GetComponentLocation` (`self.PlaceBallSpawn`)))) (struct) (`self.SpawnScaleBall`)) "AlwaysSpawn" "OverrideRootScale" null null))))
      (return))))

(fn `StopCarriage`
  (set `self.MoveLeftDeltaLocation` (0.0 0.0 0.0))
  (set `self.MoveRightDeltaLocation` (0.0 0.0 0.0))
  (return))

(fn `StopGame`
  (bind _returnvalue (`GameplayStatics.GetPlayerController` 0))
  (`self.DeletePlayableActors`)
  (`/Game/Arkanoid/Core/GameObjects/BP_GameBall.StopBall` (`self.GameBall`))
  (`self.StopCarriage` self)
  (if (> (`self.BallLives`) 0)
    (bind _returnvalue_2 (`KismetSystemLibrary.K2_SetTimer` null "RunWinWidget" 1.5))
    (set `self.TimerStopGame` _returnvalue_2)
    (else
      (bind _returnvalue_3 (`KismetSystemLibrary.K2_SetTimer` null "RunLoseWidget" 1.5))
      (set `self.TimerStopGame` _returnvalue_3)))
  (`/Engine/EditorBlueprintResources/StandardMacros.IsValid` _returnvalue
    (:`Is Valid`
      (`WidgetBlueprintLibrary.SetInputMode_UIOnlyEx` _returnvalue null)
      (set `PlayerController.bShowMouseCursor` true (`GameplayStatics.GetPlayerController` 0))
      (`KismetSystemLibrary.K2_ClearAndInvalidateTimerHandle` (`self.TimerShowWidgets`))
      (return))))

(fn `UserConstructionScript`)