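; BP_ExtraBall is an extra ball actor for the Arkanoid game that bounces around the scene.
; Tick moves it with a swept local offset and reflects its direction on blocking hits, dropping the normal's Z to keep it in play.
; SetDirection randomly picks one of three launch vectors, though nothing in this Blueprint calls it.
; BeginPlay tints a dynamic material, and overlapping a KillZVolume destroys the ball.
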(event `self.ReceiveBeginPlay`
  (bind _returnvalue (`PrimitiveComponent.CreateDynamicMaterialInstance` (`self.ExtraBall`) 0 null "None"))
  (bind _output_get (set `self.MaterialInstance` _returnvalue))
  (`MaterialInstanceDynamic.SetVectorParameterValue` _output_get (`self.MaterialInstanceParameter`) (`self.MaterialInstanceColor`)))

(event `self.ReceiveActorBeginOverlap`
  (params (OtherActor :type "Actor Object Reference"))
  (cast `KillZVolume` OtherActor)
  (`self.K2_DestroyActor` self))

(event `self.ReceiveTick`
  (params (DeltaSeconds :type "Float (single-precision)"))
  (bind _sweephitresult (`SceneComponent.K2_AddLocalOffset` (`self.ExtraBall`) (* (* (`self.Direction`) (`self.Speed`)) DeltaSeconds) true false))
  (bind (_bblockinghit _binitialoverlap _time _distance _location _impactpoint _normal) (`GameplayStatics.BreakHitResult` _sweephitresult))
  (if _bblockinghit
    (set `self.Direction` (`KismetMathLibrary.GetReflectionVector` (`self.Direction`) (`KismetMathLibrary.MakeVector` (.x _normal) (.y _normal))))))

(fn `SetDirection`
  (switch `int` (`KismetMathLibrary.RandomIntegerInRange` 0 2)
    (:`0`
      (set `self.Direction` (100.0 100.0 0.0)))
    (:`1`
      (set `self.Direction` (0.0 150.0 0.0)))
    (:`2`
      (set `self.Direction` (-100.0 100.0 0.0))))
  (return))

(fn `UserConstructionScript`)