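; Arkanoid ball actor that bounces around the playfield, carries double-damage and double-speed states, and dies on overlapping a KillZVolume.
; While running, Tick moves the Ball component with a swept offset, reflecting direction off blocking hits with random X jitter and zeroed Z.
; Double damage counts down per BP_BaseBlock hit, broadcasting changes.
; Kill overlap resets both boosts, broadcasts death and destroys the actor.
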(event `self.ReceiveHit`
  (params (MyComp :type "PrimitiveComponent Object Reference") (Other :type "Actor Object Reference") (OtherComp :type "PrimitiveComponent Object Reference") (bSelfMoved :type Boolean) (HitLocation :type "Vector Structure") (HitNormal :type "Vector Structure") (NormalImpulse :type "Vector Structure") (Hit :type "HitResult Structure (by ref)"))
  (cast `/Game/Arkanoid/Core/Blocks/BP_BaseBlock` Other)
  (bind _doubledamage (`self.GetDoubleDamageInfo`))
  (if _doubledamage
    (`/Engine/EditorBlueprintResources/StandardMacros.DecrementInt` (`self.DoubleDamageAmountBlocks`)
      (:`  `
        (`self.OnDoubleDamageCountChanged`)
        (if (== (`self.DoubleDamageAmountBlocks`) 0)
          (`self.UnsetDoubleDamage`))))))

(event `self.ReceiveActorBeginOverlap`
  (params (OtherActor :type "Actor Object Reference"))
  (cast `KillZVolume` OtherActor)
  (`self.UnsetDoubleDamage`)
  (`self.SetDefaultSpeed`)
  (`self.OnDeath`)
  (`self.K2_DestroyActor` self)
  (`self.StopBall`))

(event `self.ReceiveBeginPlay`
  (bind _returnvalue (`PrimitiveComponent.CreateDynamicMaterialInstance` (`self.Ball`) 0 null "None"))
  (bind _output_get (set `self.MaterialInstance` _returnvalue))
  (`MaterialInstanceDynamic.SetVectorParameterValue` _output_get (`self.ParameterMaterialInstance`) (`self.ColorMaterialInstance`))
  (set `self.DefaultSpeed` (`self.Speed`)))

(event `self.ReceiveTick`
  (params (DeltaSeconds :type "Float (single-precision)"))
  (bind _isrun (`self.GetInfoBallRunning`))
  (if _isrun
    (bind _sweephitresult (`SceneComponent.K2_AddLocalOffset` (`self.Ball`) (* (* (`self.Direction`) (`self.Speed`)) DeltaSeconds) true false))
    (bind (_bblockinghit _binitialoverlap _time _distance _location _impactpoint _normal) (`GameplayStatics.BreakHitResult` _sweephitresult))
    (if _bblockinghit
      (set `self.Direction` (`KismetMathLibrary.MakeVector` (+ (`KismetMathLibrary.RandomFloatInRange` -25.0 25.0) (.x (`KismetMathLibrary.GetReflectionVector` (`self.Direction`) (`KismetMathLibrary.MakeVector` (.x _normal) (.y _normal))))) (.y (`KismetMathLibrary.GetReflectionVector` (`self.Direction`) (`KismetMathLibrary.MakeVector` (.x _normal) (.y _normal)))))))))

(fn `GetDoubleDamageCount`
  (returns (DoubleDamageCount :type Integer))
  (return (`self.DoubleDamageAmountBlocks`)))

(fn `GetDoubleDamageInfo`
  (returns (DoubleDamage :type Boolean))
  (return (`self.IsDoubleDamage`)))

(fn `GetInfoBallRunning`
  (returns (IsRun :type Boolean))
  (return (`self.IsBallRun`)))

(fn `GetInfoDoubleUpSpeed`
  (returns (DoubleSpeed :type Boolean))
  (return (`self.IsDoubleUpSpeed`)))

(fn `RunBall`
  (set `self.IsBallRun` true)
  (`self.SetDefaultSpeed`)
  (return))

(fn `SetDefaultSpeed`
  (set `self.Speed` (`self.DefaultSpeed`))
  (set `self.IsDoubleUpSpeed` false)
  (return))

(fn `SetDoubleDamage`
  (bind _doubledamage (`self.GetDoubleDamageInfo`))
  (if _doubledamage
    (set `self.DoubleDamageAmountBlocks` 5)
    (else
      (set `self.IsDoubleDamage` true)
      (set `self.DoubleDamageAmountBlocks` 5)))
  (`self.OnDoubleDamageCountChanged`)
  (return))

(fn `SetDoubleUpSpeed`
  (bind _doublespeed (`self.GetInfoDoubleUpSpeed`))
  (if (not _doublespeed)
    (set `self.Speed` (* (`self.Speed`) 2.0))
    (set `self.IsDoubleUpSpeed` true))
  (return))

(fn `StopBall`
  (set `self.IsBallRun` false)
  (set `self.Speed` 0.0)
  (return))

(fn `UnsetDoubleDamage`
  (bind _doubledamage (`self.GetDoubleDamageInfo`))
  (if _doubledamage
    (set `self.IsDoubleDamage` false)
    (set `self.DoubleDamageAmountBlocks` 0)
    (`self.OnDoubleDamageCountChanged`)
    (return)))

(fn `UserConstructionScript`)