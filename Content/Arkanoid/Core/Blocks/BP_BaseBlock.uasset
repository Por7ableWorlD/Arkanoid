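; Base Arkanoid block that loses lives when hit by the game ball or an extra ball and can drop a bonus when destroyed.
; A dynamic material instance shows remaining lives as a color through SetColour.
; The game ball removes an additional life when double damage is active.
; At zero lives it destroys itself, calls CallOnDestroy and runs chained weighted rolls to spawn at most one power-up or penalty pickup.
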(event `self.ReceiveBeginPlay`
  (bind _returnvalue (`PrimitiveComponent.CreateDynamicMaterialInstance` (`self.Block`) 0 null "None"))
  (set `self.MaterialInstanceBlock` _returnvalue)
  (`self.SetColour` (`self.Lives`)))

(event `self.ReceiveHit`
  (params (MyComp :type "PrimitiveComponent Object Reference") (Other :type "Actor Object Reference") (OtherComp :type "PrimitiveComponent Object Reference") (bSelfMoved :type Boolean) (HitLocation :type "Vector Structure") (HitNormal :type "Vector Structure") (NormalImpulse :type "Vector Structure") (Hit :type "HitResult Structure (by ref)"))
  (bind _asbp_game_ball (cast `/Game/Arkanoid/Core/GameObjects/BP_GameBall` Other)
    (:`then`
      (bind _output_get (set `self.GameBall` _asbp_game_ball))
      (bind _doubledamage (`/Game/Arkanoid/Core/GameObjects/BP_GameBall.GetDoubleDamageInfo` _output_get))
      (if _doubledamage
        (`/Engine/EditorBlueprintResources/StandardMacros.DecrementInt` (`self.Lives`)
          (:`  `
            _))))
    (:`CastFailed`
      (bind _asbp_extra_ball (cast `/Game/Arkanoid/Core/GameObjects/BP_ExtraBall` Other))
      (set `self.ExtraBall` _asbp_extra_ball)))
  (bind _result (`/Engine/EditorBlueprintResources/StandardMacros.DecrementInt` (`self.Lives`))
    (:`  `
      (if (<= _result 0)
        (set `self.SpawnLocationBonus` (`SceneComponent.K2_GetComponentLocation` (`self.Block`)))
        (`self.K2_DestroyActor` self)
        (`self.OnDestroy`)
        (if (`KismetMathLibrary.RandomBoolWithWeight` (`self.DoubleDamageSpawnChance`))
          (`|SpawnActorFromClass` "/Game/Arkanoid/Core/Bonuses/Positive/BP_DoubleDamageBall.BP_DoubleDamageBall_C" (`KismetMathLibrary.MakeTransform` (`self.SpawnLocationBonus`) (struct) (`self.SpawnScaleBonus`)) "Undefined" "OverrideRootScale" null null)
          (elif (`KismetMathLibrary.RandomBoolWithWeight` (`self.ExtraBallSpawnChance`))
            (`|SpawnActorFromClass` "/Game/Arkanoid/Core/Bonuses/Positive/BP_AddBall.BP_AddBall_C" (`KismetMathLibrary.MakeTransform` (`self.SpawnLocationBonus`) (struct) (`self.SpawnScaleBonus`)) "AlwaysSpawn" "OverrideRootScale" null null)
            (elif (`KismetMathLibrary.RandomBoolWithWeight` (`self.DoubleUpSpeedBallChance`))
              (`|SpawnActorFromClass` "/Game/Arkanoid/Core/Bonuses/Positive/BP_DoubleUpSpeedBall.BP_DoubleUpSpeedBall_C" (`KismetMathLibrary.MakeTransform` (`self.SpawnLocationBonus`) (struct) (`self.SpawnScaleBonus`)) "AlwaysSpawn" "OverrideRootScale" null null)
              (elif (`KismetMathLibrary.RandomBoolWithWeight` (`self.DoubleUpSpeedCarriageChance`))
                (`|SpawnActorFromClass` "/Game/Arkanoid/Core/Bonuses/Positive/BP_DoubleUpSpeedCarriage.BP_DoubleUpSpeedCarriage_C" (`KismetMathLibrary.MakeTransform` (`self.SpawnLocationBonus`) (struct) (`self.SpawnScaleBonus`)) "AlwaysSpawn" "OverrideRootScale" null null)
                (elif (`KismetMathLibrary.RandomBoolWithWeight` (`self.RemoveOneBallLiveChance`))
                  (`|SpawnActorFromClass` "/Game/Arkanoid/Core/Bonuses/Negative/BP_RemoveOneBallLife.BP_RemoveOneBallLife_C" (`KismetMathLibrary.MakeTransform` (`self.SpawnLocationBonus`) (struct) (`self.SpawnScaleBonus`)) "AlwaysSpawn" "OverrideRootScale" null null)
                  (elif (`KismetMathLibrary.RandomBoolWithWeight` (`self.DoubleDownSpeedCarriageChance`))
                    (`|SpawnActorFromClass` "/Game/Arkanoid/Core/Bonuses/Negative/BP_DoubleDownSpeedCarriage.BP_DoubleDownSpeedCarriage_C" (`KismetMathLibrary.MakeTransform` (`self.SpawnLocationBonus`) (struct) (`self.SpawnScaleBonus`)) "AlwaysSpawn" "OverrideRootScale" null null)
                    (elif (`KismetMathLibrary.RandomBoolWithWeight` (`self.AddOneBallLiveChance`))
                      (`|SpawnActorFromClass` "/Game/Arkanoid/Core/Bonuses/Positive/BP_AddOneBallLife.BP_AddOneBallLife_C" (`KismetMathLibrary.MakeTransform` (`self.SpawnLocationBonus`) (struct) (`self.SpawnScaleBonus`)) "AlwaysSpawn" "OverrideRootScale" null null))))))))
        (else
          (`self.SetColour` (`self.Lives`)))))))

(fn `SetColour`
  (params (BlockLives :type Integer))
  (switch `int` BlockLives
    (:`1`
      (bind _output_get (set `self.MaterialInstanceColorBlock` (struct :`R` 1.0 :`G` 0.972549 :`A` 1.0)))
      (`MaterialInstanceDynamic.SetVectorParameterValue` (`self.MaterialInstanceBlock`) (`self.MaterialInstanceParameterBlock`) _output_get))
    (:`2`
      (bind _output_get_2 (set `self.MaterialInstanceColorBlock` (struct :`G` 1.0 :`A` 1.0)))
      (`MaterialInstanceDynamic.SetVectorParameterValue` (`self.MaterialInstanceBlock`) (`self.MaterialInstanceParameterBlock`) _output_get_2))
    (:`3`
      (bind _output_get_3 (set `self.MaterialInstanceColorBlock` (struct :`B` 1.0 :`A` 1.0)))
      (`MaterialInstanceDynamic.SetVectorParameterValue` (`self.MaterialInstanceBlock`) (`self.MaterialInstanceParameterBlock`) _output_get_3))
    (:`4`
      (bind _output_get_4 (set `self.MaterialInstanceColorBlock` (struct :`R` 1.0 :`A` 1.0)))
      (`MaterialInstanceDynamic.SetVectorParameterValue` (`self.MaterialInstanceBlock`) (`self.MaterialInstanceParameterBlock`) _output_get_4)))
  (return))

(fn `UserConstructionScript`)