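; Base breakable block that counts hits from BP_GameBall and destroys its Cube component, not the actor, once Hits reaches Lives.
; SetColour runs at BeginPlay and after each non-final hit, creating a dynamic material instance to set the Cube's Colour parameter from Lives.
; Lives itself never decrements here, so the colour reflects the configured Lives rather than the hits remaining.
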(event `self.ReceiveBeginPlay`
  (`self.SetColour`))

(event `self.ReceiveHit`
  (params (MyComp :type "PrimitiveComponent Object Reference") (Other :type "Actor Object Reference") (OtherComp :type "PrimitiveComponent Object Reference") (bSelfMoved :type Boolean) (HitLocation :type "Vector Structure") (HitNormal :type "Vector Structure") (NormalImpulse :type "Vector Structure") (Hit :type "HitResult Structure (by ref)"))
  (cast `/Game/Core/Blueprints/BP_GameBall` Other)
  (bind _result (`/Engine/EditorBlueprintResources/StandardMacros.IncrementInt` (`self.Hits`))
    (:`  `
      (if (== _result (`self.Lives`))
        (`ActorComponent.K2_DestroyComponent` (`self.Cube`))
        (else
          (`self.SetColour`))))))

(fn `SetColour`
  (locals (Colour :type "LinearColor Structure"))
  (if (== (`self.Lives`) 1)
    (set `local.Colour` (struct :`R` 1.0 :`G` 0.969542 :`A` 1.0))
    (bind _returnvalue (`PrimitiveComponent.CreateDynamicMaterialInstance` (`self.Cube`) 0 null "None"))
    (`MaterialInstanceDynamic.SetVectorParameterValue` _returnvalue "Colour" (`local.Colour`))
    (elif (== (`self.Lives`) 2)
      (set `local.Colour` (`KismetMathLibrary.LinearColor_Green`))
      (bind _returnvalue_2 (`PrimitiveComponent.CreateDynamicMaterialInstance` (`self.Cube`) 0 null "None"))
      (`MaterialInstanceDynamic.SetVectorParameterValue` _returnvalue_2 "Colour" (`local.Colour`))
      (elif (== (`self.Lives`) 3)
        (set `local.Colour` (`KismetMathLibrary.LinearColor_Blue`))
        (bind _returnvalue_3 (`PrimitiveComponent.CreateDynamicMaterialInstance` (`self.Cube`) 0 null "None"))
        (`MaterialInstanceDynamic.SetVectorParameterValue` _returnvalue_3 "Colour" (`local.Colour`))
        (else
          (set `local.Colour` (`KismetMathLibrary.LinearColor_Red`))
          (bind _returnvalue_4 (`PrimitiveComponent.CreateDynamicMaterialInstance` (`self.Cube`) 0 null "None"))
          (`MaterialInstanceDynamic.SetVectorParameterValue` _returnvalue_4 "Colour" (`local.Colour`)))))))

(fn `UserConstructionScript`)