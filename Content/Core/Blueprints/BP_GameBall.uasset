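; BP_GameBall is a ball actor that moves in a straight line and bounces off whatever it hits.
; On BeginPlay it creates a dynamic material instance on the Ball component and tints it cyan.
; Each Tick it moves Ball by Direction and Speed with a swept local offset, without physics simulation.
; On a blocking hit, GetReflectionVector computes the new Direction from the surface normal's X and Y.
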(event `self.ReceiveBeginPlay`
  (bind _returnvalue (`PrimitiveComponent.CreateDynamicMaterialInstance` (`self.Ball`) 0 null "None"))
  (`MaterialInstanceDynamic.SetVectorParameterValue` _returnvalue "Colour" (struct :`R` 0.003805 :`G` 1.0 :`B` 0.890338 :`A` 1.0)))

(event `self.ReceiveTick`
  (params (DeltaSeconds :type "Float (single-precision)"))
  (bind _sweephitresult (`SceneComponent.K2_AddLocalOffset` (`self.Ball`) (* (* (`self.Direction`) (`self.Speed`)) DeltaSeconds) true false))
  (bind (_bblockinghit _binitialoverlap _time _distance _location _impactpoint _normal) (`GameplayStatics.BreakHitResult` _sweephitresult))
  (if _bblockinghit
    (set `self.Direction` (`KismetMathLibrary.GetReflectionVector` (`self.Direction`) (`KismetMathLibrary.MakeVector` (.x _normal) (.y _normal))))))

(fn `UserConstructionScript`)